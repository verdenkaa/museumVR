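; Grabbable VR handler that presents a fan of color, pattern, decal, mesh or teleporter options in the ArchVisVR project.
; Options spawn as OptionBase_BP child actors, spread alternately across a wide angle and follow the handler's grab state, with a decal projector for decal sets.
; A timeline fades the dynamic material in before projecting options and reverses on close.
; When released, Tick eases the handler's roll back to level.
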(event `/Game/ArchVisVR/Blueprints/ArchVis_Interface.Pickup`
  (params (AttachTo :type "SceneComponent Object Reference"))
  ;[1 1 1] Pickup and drop handler
  (`self.GrabOptions` true)
  (`SceneComponent.K2_AttachToComponent` (`self.K2_GetRootComponent`) AttachTo "None" "KeepWorld" "KeepWorld" "KeepWorld" true)
  (set `self.bGrabed` true))

(event `/Game/ArchVisVR/Blueprints/ArchVis_Interface.Drop`
  ;[1 1 1] Pickup and drop handler
  (`self.GrabOptions` false)
  (`self.K2_DetachFromActor` "KeepWorld" "KeepWorld" "KeepWorld")
  (set `self.bGrabed` false))

(event `self.ReceiveTick`
  (params (DeltaSeconds :type "Float (single-precision)"))
  ;[1 1 1] Set rotation
  (if (not (`self.bGrabed`))
    (`self.K2_SetActorRotation` (`KismetMathLibrary.MakeRotator` (`KismetMathLibrary.FInterpTo` (.roll (`self.K2_GetActorRotation`)) 0.0 DeltaSeconds 2.5) (.pitch (`self.K2_GetActorRotation`)) (.yaw (`self.K2_GetActorRotation`))))))

(event `self.ReceiveBeginPlay`
  (bind _mid (`self.MID`))
  ;[1 1 1] Opening and closing animation effect
  (bind _returnvalue (`PrimitiveComponent.CreateDynamicMaterialInstance` (`self.Mesh`) 0 "/Game/ArchVisVR/Materials/Handler/M_Handler_Base.M_Handler_Base"))
  (set `self.MID` _returnvalue)
  (`SkeletalMeshComponent.PlayAnimation` (`self.Mesh`) "/Game/ArchVisVR/Meshes/OptionHandler_SK_Anim.OptionHandler_SK_Anim" false)
  (bind (_direction _opacity _static) (`Timeline|OpeningEffect` :!via `PlayFromStart` :!label _label)
    (:`Update`
      (`MaterialInstanceDynamic.SetScalarParameterValue` _mid "GlobalOpacity" _opacity)
      (`MaterialInstanceDynamic.SetScalarParameterValue` _mid "Static" _static))
    (:`Finished`
      (`KismetSystemLibrary.Delay` 0.5)
      (for _array_element (`self.Options`)
        (bind _asoption_base_bp (cast `/Game/ArchVisVR/Blueprints/Option/OptionBase_BP` (`ChildActorComponent.ChildActor` _array_element)))
        (set `/Game/ArchVisVR/Blueprints/Option/OptionBase_BP.bProjected` true _asoption_base_bp)))))

(event `DestroyEffect`
  ;[1 1 1] Opening and closing animation effect
  (goto _label :!via `ReverseFromEnd`))

(fn `AddOptionChildComponent`
  (returns (NewChildOption :type "ChildActorComponent Object Reference"))
  (bind (_returnvalue_x _returnvalue_y _returnvalue_z) (`KismetMathLibrary.BreakVector` (`self.K2_GetActorLocation`)))
  (bind _returnvalue (`AddComponent|NODE_AddChildActorComponent-1` :`bManualAttachment` true :`RelativeTransform` (`KismetMathLibrary.MakeTransform` (`KismetMathLibrary.MakeVector` _returnvalue_x _returnvalue_y (- _returnvalue_z 15.0)) (`self.K2_GetActorRotation`) (`self.OptionsScale`))))
  (return _returnvalue))

(fn `CloseOptions`
  (bind _decalhandler (`self.DecalHandler`))
  ;[1 1 1] Destroy option actors
  (for _array_element (`self.Options`)
    (`ActorComponent.K2_DestroyComponent` _array_element))
  ;[1 1 1] Remove all options from array
  (`KismetArrayLibrary.Array_Clear` (`self.Options`))
  ;[1 1 1] Remove decal projector
  (`/Engine/EditorBlueprintResources/StandardMacros.IsValid` _decalhandler
    (:`Is Valid`
      (`self.K2_DestroyActor` _decalhandler))
    (:`Is Not Valid`
      _))
  ;[1 1 1] Closing effec
  (`TimelineComponent.ReverseFromEnd` (`self.OpeningEffect`))
  (`self.SetLifeSpan` 2.0))

(fn `GrabOptions`
  (params (bGrab :type Boolean))
  ;[1 1 1] Set grabbed on the options to move to default location
  (for _array_element (`self.Options`)
    (bind _asoption_base_bp (cast `/Game/ArchVisVR/Blueprints/Option/OptionBase_BP` (`ChildActorComponent.ChildActor` _array_element)))
    (set `/Game/ArchVisVR/Blueprints/Option/OptionBase_BP.bGrabed` bGrab _asoption_base_bp)))

(fn `SetOptionLocationAndRotation`
  (locals (Degree :type "Float (double-precision)" :default 0.0))
  (bind _options (`self.Options`))
  (bind _returnvalue (`KismetArrayLibrary.Array_Length` (`self.Options`)))
  ;[1 1 1] Set options location and rotation depends on numbers of options and wide angle of handler
  (set `local.Degree` (/ (`self.OptionWideDegree`) (`KismetMathLibrary.Conv_IntToDouble` _returnvalue)))
  (if (> _returnvalue 1)
    (for _index (range 1 (`KismetArrayLibrary.Array_Length` _options))
      (bind _returnvalue_2 (== (mod _index 2) 0))
      (bind _asoption_base_bp (cast `/Game/ArchVisVR/Blueprints/Option/OptionBase_BP` (`ChildActorComponent.ChildActor` (`KismetArrayLibrary.Array_Get` _options (`KismetMathLibrary.SelectInt` (- _index 2) (- _index 1) _returnvalue_2)))))
      (bind _item (`KismetArrayLibrary.Array_Get` _options _index))
      (bind _asoption_base_bp_2 (cast `/Game/ArchVisVR/Blueprints/Option/OptionBase_BP` (`ChildActorComponent.ChildActor` _item)))
      (bind _output_get (set `/Game/ArchVisVR/Blueprints/Option/OptionBase_BP.DesiredDegree` (* (- (`/Game/ArchVisVR/Blueprints/Option/OptionBase_BP.DesiredDegree` _asoption_base_bp) (`local.Degree`)) (`KismetMathLibrary.SelectFloat` 1.0 -1.0 _returnvalue_2)) _asoption_base_bp_2))
      (bind _output_get_2 (set `/Game/ArchVisVR/Blueprints/Option/OptionBase_BP.DesiredLocation` (- (`SceneComponent.K2_GetComponentLocation` _item) (`KismetMathLibrary.MakeVector` (* (`KismetMathLibrary.Conv_IntToDouble` _index) 0.5 -1.0))) _asoption_base_bp_2)))
    ;[1 1 1] Attach options to handler
    (for _array_element (`self.Options`)
      (`SceneComponent.K2_AttachToComponent` _array_element (`self.Root`) "None" "KeepWorld" "KeepWorld" "KeepWorld" true))
    ;[1 1 1] Spawn Decal projector
    (switch `/Game/ArchVisVR/Blueprints/Option/OptionType/ArchVisVR_Options` (`self.OptionType`)
      (:`NewEnumerator2`
        (`self.SpawnDecalHandler`)))))

(fn `SpawnDecalHandler`
  ;[1 1 1] Spawn decal projector at decal projector location from mesh
  (bind _asarch_vis_vr_base_actor_bp (cast `/Game/ArchVisVR/Blueprints/Actor/ArchVisVR_BaseActor_BP` (`self.GetOwner`)))
  (bind _decalprojectorlocation (`/Game/ArchVisVR/Blueprints/Actor/ArchVisVR_BaseActor_BP.DecalProjectorLocation` _asarch_vis_vr_base_actor_bp))
  (bind _returnvalue (`|SpawnActorFromClass` "/Game/ArchVisVR/Blueprints/Option/DecalHandler_BP.DecalHandler_BP_C" (`KismetMathLibrary.MakeTransform` (`SceneComponent.K2_GetComponentLocation` _decalprojectorlocation) (`SceneComponent.K2_GetComponentRotation` _decalprojectorlocation)) "Undefined" "OverrideRootScale" null _asarch_vis_vr_base_actor_bp))
  (set `self.DecalHandler` _returnvalue))

(fn `SpawnOptions`
  (params (NewColorInfo :type "/Game/ArchVisVR/Blueprints/Option/OptionType/ArchVisVR_ColorOption Structure") (NewPatternInfo :type "/Game/ArchVisVR/Blueprints/Option/OptionType/ArchVisVR_PatternOption Structure") (NewDecalInfo :type "/Game/ArchVisVR/Blueprints/Option/OptionType/ArchVisVR_DecalOption Structure") (NewMeshInfo :type "/Game/ArchVisVR/Blueprints/Option/OptionType/ArchVisVR_MeshOption Structure") (NewTeleporterInfo :type "/Game/ArchVisVR/Blueprints/Option/OptionType/ArchVisVR_TeleporterOption Structure") (NewUIStyle :type "/Game/ArchVisVR/Blueprints/Option/OptionType/ArchVisVR_UIStyle Structure"))
  (bind (_returnvalue_x _returnvalue_y _returnvalue_z) (`KismetMathLibrary.BreakVector` (`self.K2_GetActorLocation`)))
  (bind _options (`self.Options`))
  ;[1 1 1] Spawn options depends on what type of option they must be
  (bind _newchildoption (`self.AddOptionChildComponent`))
  (bind _returnvalue (`KismetArrayLibrary.Array_Add` _options _newchildoption))
  (bind _asoption_base_bp (cast `/Game/ArchVisVR/Blueprints/Option/OptionBase_BP` (`ChildActorComponent.ChildActor` (`KismetArrayLibrary.Array_Get` _options _returnvalue))))
  (set `/Game/ArchVisVR/Blueprints/Option/OptionBase_BP.DesiredLocation` (`KismetMathLibrary.MakeVector` _returnvalue_x _returnvalue_y (- _returnvalue_z 15.0)) _asoption_base_bp)
  (`/Game/ArchVisVR/Blueprints/Option/OptionBase_BP.SetOptionType` _asoption_base_bp (`self.OptionType`))
  (`/Game/ArchVisVR/Blueprints/Option/OptionBase_BP.SetUIStyle` _asoption_base_bp NewUIStyle)
  (switch `/Game/ArchVisVR/Blueprints/Option/OptionType/ArchVisVR_Options` (`self.OptionType`)
    (:`NewEnumerator0`
      (`/Game/ArchVisVR/Blueprints/Option/OptionBase_BP.OptionToShow` :`self` _asoption_base_bp :`NewColorInfo` NewColorInfo))
    (:`NewEnumerator1`
      (`/Game/ArchVisVR/Blueprints/Option/OptionBase_BP.OptionToShow` :`self` _asoption_base_bp :`NewPatternInfo` NewPatternInfo))
    (:`NewEnumerator2`
      (`/Game/ArchVisVR/Blueprints/Option/OptionBase_BP.OptionToShow` :`self` _asoption_base_bp :`NewDecalInfo` NewDecalInfo))
    (:`NewEnumerator3`
      (`/Game/ArchVisVR/Blueprints/Option/OptionBase_BP.OptionToShow` :`self` _asoption_base_bp :`NewMeshInfo` NewMeshInfo))
    (:`NewEnumerator5`
      (`/Game/ArchVisVR/Blueprints/Option/OptionBase_BP.OptionToShow` :`self` _asoption_base_bp :`NewTeleporterInfo` NewTeleporterInfo))))

(fn `UserConstructionScript`)