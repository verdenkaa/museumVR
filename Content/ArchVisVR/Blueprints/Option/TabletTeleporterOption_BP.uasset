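; A selectable option on the ArchVis VR tablet that represents one teleport destination.
; InitializeOption stores the teleport info and target transform, then shows the destination's picture on the option mesh through a dynamic material instance.
; ActivateOption finds the tablet as its parent actor and the tablet's owning VR pawn, then tells that pawn to teleport to the stored transform.
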(fn `ActivateOption`
  (bind _asarch_vis_tablet_bp (cast `/Game/ArchVisVR/Blueprints/Player/ArchVis_Tablet_BP` (`self.GetParentActor`)))
  (bind _asarch_vis_vrpawn_bp (cast `/Game/ArchVisVR/Blueprints/Player/ArchVis_VRPawn_BP` (`self.GetOwner` _asarch_vis_tablet_bp)))
  (`/Game/ArchVisVR/Blueprints/Player/ArchVis_VRPawn_BP.TabletTeleportTo` _asarch_vis_vrpawn_bp (`self.TeleporterTransform`)))

(fn `InitializeOption`
  (params (NewOption :type "/Game/ArchVisVR/Blueprints/Option/OptionType/ArchVisVR_TeleporterOption Structure") (TeleporterTransform :type "Transform Structure"))
  (bind _output_get (set `self.TeleportInfo` NewOption))
  (set `self.TeleporterTransform` TeleporterTransform)
  (bind _returnvalue (`PrimitiveComponent.CreateDynamicMaterialInstance` (`self.OptionMesh`) 1 "/Game/ArchVisVR/Materials/Option/MI_TabletOption.MI_TabletOption"))
  (`PrimitiveComponent.SetMaterial` (`self.OptionMesh`) 1 _returnvalue)
  (`MaterialInstanceDynamic.SetTextureParameterValue` _returnvalue "BaseTexture" (`.Picture_2_4096544949A3076D8CBC0FACC53E31E3` (break `/Game/ArchVisVR/Blueprints/Option/OptionType/ArchVisVR_TeleporterOption` _output_get))))

(fn `UserConstructionScript`)