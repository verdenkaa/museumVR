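; A VR-grabbable decal projector handle that positions a decal on a target ArchVis base actor.
; Pickup attaches it to the given component and Drop detaches it, keeping world transforms.
; Every Tick it line-traces along its Arrow on the Visibility channel.
; When the trace hits TargetActor, it passes projector location and rotation, hit point and distance to that actor's UpdateDecal.
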(event `/Game/ArchVisVR/Blueprints/ArchVis_Interface.Pickup`
  (params (AttachTo :type "SceneComponent Object Reference"))
  ;[1 1 1] Pickup and move decal projector
  (`self.K2_AttachToComponent` self AttachTo "None" "KeepWorld" "KeepWorld" "KeepWorld" false))

(event `/Game/ArchVisVR/Blueprints/ArchVis_Interface.Drop`
  ;[1 1 1] Pickup and move decal projector
  (`self.K2_DetachFromActor` "KeepWorld" "KeepWorld" "KeepWorld"))

(event `self.ReceiveTick`
  (params (DeltaSeconds :type "Float (single-precision)"))
  (bind _returnvalue (`self.K2_GetActorLocation`))
  (bind _arrow (`self.Arrow`))
  (bind _returnvalue_2 (`SceneComponent.K2_GetComponentLocation` _arrow))
  ;[1 1 1] Update decal location and size depends on distance to mesh and projector location
  (bind (_outhit _returnvalue_3) (`KismetSystemLibrary.LineTraceSingle` _returnvalue_2 (+ _returnvalue_2 (* (`SceneComponent.GetForwardVector` _arrow) (`self.TraceDistance`))) "TraceTypeQuery1"))
  (`/Engine/EditorBlueprintResources/StandardMacros.IsValid` (`self.TargetActor`)
    (:`Is Valid`
      (if _returnvalue_3
        (bind (_bblockinghit _binitialoverlap _time _location _impactpoint _normal _impactnormal _physmat _hitactor) (`GameplayStatics.BreakHitResult` _outhit))
        (bind (_asarch_vis_vr_base_actor_bp _bsuccess) (cast `/Game/ArchVisVR/Blueprints/Actor/ArchVisVR_BaseActor_BP` _hitactor :!pure true))
        (if (and (== (`self.TargetActor`) _asarch_vis_vr_base_actor_bp) _bsuccess)
          (`/Game/ArchVisVR/Blueprints/Actor/ArchVisVR_BaseActor_BP.UpdateDecal` (`self.TargetActor`) _returnvalue (`KismetMathLibrary.VSize` (- _location _returnvalue)) _location (`self.K2_GetActorRotation`)))))))

(fn `UserConstructionScript`)