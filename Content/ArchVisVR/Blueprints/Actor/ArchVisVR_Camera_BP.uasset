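; A hand-held camera actor for the ArchVis VR project that takes screenshots from its own viewpoint.
; Pickup attaches it to the given component and registers it with the VR pawn; Drop detaches and unregisters it.
; TakeShot switches the player's view target to this camera and fires the HighResShot console command.
; The Active flag blocks repeat shots until a short timer calls BackToNormal, which resets the pawn's camera.
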(event `self.ReceiveBeginPlay`
  (`self.SetOwner` (`GameplayStatics.GetPlayerController` 0)))

(event `/Game/ArchVisVR/Blueprints/ArchVis_Interface.Pickup`
  (params (AttachTo :type "SceneComponent Object Reference"))
  ;[1 1 1] Pickup or drop camera
  ;;[1 1 1] Attch to hand and set as camera class in pawn class
  (`SceneComponent.K2_AttachToComponent` (`self.K2_GetRootComponent`) AttachTo "None" "KeepWorld" "KeepWorld" "KeepWorld" true)
  (bind _asarch_vis_vrpawn_bp (cast `/Game/ArchVisVR/Blueprints/Player/ArchVis_VRPawn_BP` (`GameplayStatics.GetPlayerPawn` 0)))
  (`/Game/ArchVisVR/Blueprints/Player/ArchVis_VRPawn_BP.AttachCamera` _asarch_vis_vrpawn_bp self true))

(event `/Game/ArchVisVR/Blueprints/ArchVis_Interface.Drop`
  ;[1 1 1] Pickup or drop camera
  ;;[1 1 1] Detach from hand and set pawn camera class to null
  (`self.K2_DetachFromActor` "KeepWorld" "KeepWorld" "KeepWorld")
  (bind _asarch_vis_vrpawn_bp (cast `/Game/ArchVisVR/Blueprints/Player/ArchVis_VRPawn_BP` (`GameplayStatics.GetPlayerPawn` 0)))
  (`/Game/ArchVisVR/Blueprints/Player/ArchVis_VRPawn_BP.AttachCamera` _asarch_vis_vrpawn_bp null false))

(fn `BackToNormal`
  ;[1 1 1] Back to normal pawn camera after take screenshot
  (set `self.bActive` true)
  (bind _asarch_vis_vrpawn_bp (cast `/Game/ArchVisVR/Blueprints/Player/ArchVis_VRPawn_BP` (`GameplayStatics.GetPlayerPawn` 0)))
  (`/Game/ArchVisVR/Blueprints/Player/ArchVis_VRPawn_BP.ResetCamera` _asarch_vis_vrpawn_bp))

(fn `TakeShot`
  ;[1 1 1] Take screenshot, move change pawn camera to this camera
  (if (`self.bActive`)
    (set `self.bActive` false)
    (`PlayerController.SetViewTargetWithBlend` (`GameplayStatics.GetPlayerController` 0) (`ActorComponent.GetOwner` (`self.Camera`)) 0.0 "VTBlend_Linear" 0.0 false)
    (`KismetSystemLibrary.ExecuteConsoleCommand` "HighResShot 1")
    (`KismetSystemLibrary.K2_SetTimer` self "BackToNormal" 0.5)))

(fn `UserConstructionScript`)